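; BP_Gun is an automatic hitscan weapon held by a parent actor, which can be dropped as a physics object.
; While firing, it loops on a bullet delay, tracing from the Nozzle socket to the parent's target and notifying hit actors.
; Each shot drives surface-based impact effects, a moving trail and decaying recoil sent to the parent via messages.
; Reticle accuracy follows firing state; release resets recoil and plays a shell-drop sound.
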(event EventBeginPlay)

(event Collision|EventActorBeginOverlap
  (params (OtherActor :type Actor%20Object%20Reference)))

(event EventTick
  (params (DeltaSeconds :type Float%20%28single-precision%29)))

(event EventDrop
  (bind _sk_assault_2 (Variables|Default|GetSK_Assault_2))
  (Transformation|DetachFromActor self "KeepWorld" "KeepWorld" "KeepWorld")
  (Collision|SetCollisionProfileName _sk_assault_2 "BlockAll" true :!class /Script/Engine.PrimitiveComponent)
  (Collision|SetCollisionEnabled _sk_assault_2 "QueryAndPhysics")
  (Physics|SetSimulatePhysics _sk_assault_2 true))

(fn ConstructionScript)

(event EventFire
  (params (start/stop :type Boolean))
  (bind _returnvalue (Game|GetPlayerController 0))
  (bind _p_impactspark (Variables|Default|GetP_ImpactSpark))
  (bind _returnvalue_2 (HUD|GetHUD _returnvalue))
  (bind _output_get (Variables|Default|Setfiring start/stop))
  (if _output_get :!label _label
    (Class|BPIUI|SetReticleAccuracy(Message) _returnvalue_2 0.1)
    (Components|Activation|Activate (Variables|Default|GetP_bulletshell) true)
    (Components|Activation|Activate _p_impactspark false)
    (Audio|PlaySoundatLocation "/Game/Blueprints/Guns/AK_47_Single_Shot_4_Sound_Effect__HD.AK_47_Single_Shot_4_Sound_Effect__HD" (Transformation|GetActorLocation) "0, 0, 0" 1.0 1.0 0.0 0 0 0)
    (bind _target (Class|BPICharacter|GetTargetlocationBPICh(Message) (Actor|GetParentActor)))
    (bind (_outhit _returnvalue_3) (Collision|LineTraceByChannel (Transformation|GetSocketLocation (Variables|Default|GetSK_Assault_2) "Nozzle") _target "TraceTypeQuery3" false 0 "None"))
    (Class|BPIDamageable|OnBulletHit(Message) (.hitactor _outhit))
    (if (.bblockinghit _outhit)
      (|ImpactparticleandDecal (select (.bblockinghit _outhit) (.impactpoint _outhit) _target) (.impactnormal _outhit) _returnvalue_3 (.physmat _outhit)) ; Impact particle and decal
    )
    (Class|BPICharacter|AddRecoil(Message) (Actor|GetParentActor) (Variables|Default|Getrecoil%20Rotation) (Variables|Default|Getrecoil%20Pitch%20Input))
    (Variables|Default|Setrecoil%20Pitch%20Input (* (Variables|Default|Getrecoil%20Pitch%20Input) 0.8))
    (Utilities|FlowControl|Sequence
      (:then_0
        (Utilities|FlowControl|Delay (Variables|Default|Getbullet_delay))
        (Components|Activation|Deactivate _p_impactspark)
        (goto _label))
      (:then_1
        (|Bullettrail (select (.bblockinghit _outhit) (.impactpoint _outhit) _target)) ; Bullet trail
      ))
    (else
      (Class|BPIUI|SetReticleAccuracy(Message) _returnvalue_2 0.5)
      (Variables|Default|Setrecoil%20Pitch%20Input (Variables|Default|Getrecoil%20Pitch%20Input%20Max))
      (|Bulletshellsound) ; Bullet shell sound
    )))

(fn GetWeaponSocket
  (params (socket%20name :type Name :default "None"))
  (return (Transformation|GetSocketTransform (Variables|Default|GetSK_Assault_2) socket%20name "RTS_World")))